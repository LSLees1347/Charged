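; Player pawn that handles movement, aiming and pausing through Enhanced Input, with input disabled as soon as a BP_GPPC controller possesses it.
; Move input drives movement along the actor's forward and right vectors, and aim input drives controller yaw and pitch.
; Two seconds after BeginPlay, a locally controlled pawn caches the controller's HUD widget.
; Pause toggles through BP_GameInstance, which returns whether to hide or show that HUD.
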(event Custom|DisableAllInput
  (params (PlayerController :type Player%20Controller%20Object%20Reference))
  (Input|DisableInput PlayerController))

(event Input|EnhancedActionEvents|EnhancedInputActionIA_Move
  (params (ActionValue :type Vector%202D%20Structure) (ElapsedSeconds :type Float%20%28double-precision%29) (TriggeredSeconds :type Float%20%28double-precision%29) (InputAction :type Input%20Action%20Object%20Reference :default "/Game/Input/IA_Move.IA_Move"))
  (:Triggered
    (Pawn|Input|AddMovementInput (Transformation|GetActorForwardVector) (.x ActionValue) false)
    (Pawn|Input|AddMovementInput (Transformation|GetActorRightVector) (.y ActionValue) false)))

(event Input|EnhancedActionEvents|EnhancedInputActionIA_Aim
  (params (ActionValue :type Vector%202D%20Structure) (ElapsedSeconds :type Float%20%28double-precision%29) (TriggeredSeconds :type Float%20%28double-precision%29) (InputAction :type Input%20Action%20Object%20Reference :default "/Game/Input/IA_Aim.IA_Aim"))
  (:Triggered
    (Pawn|Input|AddControllerYawInput (.x ActionValue))
    (Pawn|Input|AddControllerPitchInput (.y ActionValue))))

(event Input|EnhancedActionEvents|EnhancedInputActionIA_Pause
  (params (ActionValue :type Boolean) (ElapsedSeconds :type Float%20%28double-precision%29) (TriggeredSeconds :type Float%20%28double-precision%29) (InputAction :type Input%20Action%20Object%20Reference :default "/Game/Input/IA_Pause.IA_Pause"))
  (:Started
    (bind _asbp_game_instance (Utilities|Casting|CastToBP_GameInstance (Game|GetGameInstance)))
    (bind _result (Default|TogglePause _asbp_game_instance))
    (if _result
      (Widget|SetVisibility (Variables|Default|GetWBP_HUD) "Hidden")
      (else
        (Widget|SetVisibility (Variables|Default|GetWBP_HUD) "Visible")))))

(event EventBeginPlay
  (Utilities|FlowControl|Delay 2.0)
  (if (Pawn|IsLocallyControlled)
    (bind _asbp_gppc (Utilities|Casting|CastToBP_GPPC (Game|GetPlayerController 0)))
    (Variables|Default|SetWBP_HUD (Variables|/Game/Framework/BP_GPPC.BP_GPPC_C|GetWBP_HUD _asbp_gppc))))

(event EventPossessed
  (params (NewController :type Controller%20Object%20Reference))
  (bind _asbp_gppc (Utilities|Casting|CastToBP_GPPC NewController))
  (CallFunction|DisableAllInput _asbp_gppc))

(fn ConstructionScript)