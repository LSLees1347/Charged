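; BP_MGM is a multiplayer game mode that manages lobby players, their profiles and their lobby characters.
; Joining BP_MPC controllers are tracked and given a lobby menu, and leaving ones are removed.
; UpdateLobby copies profiles into PlayerStates, then selectively pushes names and map selection to each controller or refreshes characters.
; Players lacking a character get a named BP_LobbyPlayer spawned at the first unused BP_LobbySpot, which is marked used.
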(event Custom|UpdateLobby
  (params (PlayerNames :type Boolean) (LevelSelection :type Boolean) (CharacterSelection :type Boolean))
  (Utilities|Array|Clear (Variables|Default|GetAll_Profiles))
  (for (_array_element _array_index) (Variables|Default|GetAll_Players)
    (Utilities|Array|SetArrayElem (Variables|Default|GetAll_Profiles) _array_index (Variables|/Game/Framework/BP_MPC.BP_MPC_C|GetPlayerProfile _array_element) true)
    (bind _asbp_player_state (Utilities|Casting|CastToBP_PlayerState (Variables|/Script/Engine.Controller|GetPlayerState _array_element)))
    (Variables|/Game/Framework/BP_PlayerState.BP_PlayerState_C|SetPlayerProfile _asbp_player_state (Variables|/Game/Framework/BP_MPC.BP_MPC_C|GetPlayerProfile _array_element)))
  (for (_array_element_2 _array_index_2) (Variables|Default|GetAll_Players)
    (if PlayerNames
      (Default|UpdatePlayerNames _array_element_2 (Variables|Default|GetAll_Profiles)))
    (if LevelSelection
      (Default|UpdateLevelSelection _array_element_2 (Variables|Default|GetSelectedMap)))
    (if CharacterSelection
      (CallFunction|UpdateSelecetedChara _array_index_2))))

(event Custom|UpdateSelecetedChara
  (params (Index :type Integer))
  (bind _all_players (Variables|Default|GetAll_Players))
  (bind _output (Utilities|Array|Get(acopy) _all_players Index))
  (if (== (Variables|/Game/Framework/BP_MPC.BP_MPC_C|GetLobbyCharacter (Utilities|Array|Get(acopy) (Variables|Default|GetAll_Players) Index)) 0)
    (bind _available (CallFunction|GetLobbySpot))
    (Variables|/Game/Gameplay/Lobby/BP_LobbySpot.BP_LobbySpot_C|SetUsed? _available true)
    (bind _returnvalue (Game|SpawnActorfromClass "/Game/Gameplay/Lobby/BP_LobbyPlayer.BP_LobbyPlayer_C" (Transformation|GetActorTransform _available) "Undefined" "MultiplyWithRoot" 0 0))
    (Variables|/Game/Framework/BP_MPC.BP_MPC_C|SetLobbyCharacter _output _returnvalue)
    (Variables|/Game/Framework/BP_MPC.BP_MPC_C|SetLobbySpot _output _available)
    (Default|MCSetName (Variables|/Game/Framework/BP_MPC.BP_MPC_C|GetLobbyCharacter (Utilities|Array|Get(acopy) (Variables|Default|GetAll_Players) Index)) (Utilities|Struct|BreakS_PlayerProfile (Utilities|Array|Get(acopy) (Variables|Default|GetAll_Profiles) Index)))))

(event EventHandleStartingNewPlayer
  (params (NewPlayer :type Player%20Controller%20Object%20Reference))
  (bind _returnvalue (Game|GetCurrentLevelName true))
  (switch string _returnvalue
    (:LobbyMap
      (bind _asbp_mpc (Utilities|Casting|CastToBP_MPC NewPlayer))
      (Utilities|Array|Add (Variables|Default|GetAll_Players) _asbp_mpc)
      (Default|CreateLobbyMenu _asbp_mpc)
      (Default|Init _asbp_mpc))))

(event EventOnLogout
  (params (ExitingController :type Controller%20Object%20Reference))
  (bind _asbp_mpc (Utilities|Casting|CastToBP_MPC ExitingController))
  (Utilities|Array|RemoveItem (Variables|Default|GetAll_Players) _asbp_mpc)
  (CallFunction|UpdateLobby true false true))

(fn ConstructionScript)

(fn GetLobbySpot
  (if (== (Utilities|Array|Length (Variables|Default|GetAll_LobbySpots)) 0)
    (bind _outactors (Actor|GetAllActorsOfClass "/Game/Gameplay/Lobby/BP_LobbySpot.BP_LobbySpot_C"))
    (Variables|Default|SetAll_LobbySpots _outactors))
  (bind _array_element (Utilities|Array|ForEachLoopwithBreak (Variables|Default|GetAll_LobbySpots) :!label _label)
    (:LoopBody
      (if (not (Variables|/Game/Gameplay/Lobby/BP_LobbySpot.BP_LobbySpot_C|GetUsed? _array_element))
        (goto _label Break)))
    (:Completed
      (return _array_element))))