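; BP_MPC is the lobby player controller for a multiplayer game, managing lobby, character and loading widgets, the UI-only cursor and session exit to the main menu.
; It loads or creates the player's profile save and sends it to BP_MGM through SVR events, which refreshes the lobby or the controller's character.
; Menu switches blend the camera between pawn and lobby character, with remote clients routing that through SVR events.
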(event Custom|EndClientSession
  (|DestroySession self
    (:then
      (Game|OpenLevel(byName) "MainMenuMap "))))

(event Custom|CreateLobbyMenu
  (CallFunction|UIShowLobbyMenu))

(event Custom|SVR_SetViewTarget
  (Game|Player|SetViewTargetwithBlend (Pawn|GetControlledPawn) 0.5 "VTBlend_Linear" 0.0 false))

(event Custom|Init
  (CallFunction|LoadSaveGame)
  (CallFunction|SVRUpdateLobby (Variables|Default|GetPlayerProfile)))

(event Custom|UpdatePlayerNames
  (params (Profiles :type Array%20of%20S%20Player%20Profile%20Structures))
  (Utilities|IsValid (Variables|Default|GetWBP_Lobby)
    (:Is%20Valid
      (Default|ClearPlayerNames (Variables|Default|GetWBP_Lobby))
      (Default|UpdatePlayerNames (Variables|Default|GetWBP_Lobby) Profiles))))

(event Custom|SVR_UpdateLobby
  (params (Profile :type S%20Player%20Profile%20Structure))
  (Variables|Default|SetPlayerProfile Profile)
  (bind _asbp_mgm (Utilities|Casting|CastToBP_MGM (Game|GetGameMode)))
  (Default|UpdateLobby _asbp_mgm true true true))

(event Custom|CreateLoading
  (CallFunction|UIShowLoading))

(event Custom|UpdateLevelSelection
  (params (LevelRow :type Name))
  (Utilities|IsValid (Variables|Default|GetWBP_Lobby)
    (:Is%20Valid
      (Default|UpdateLevelSelection (Variables|Default|GetWBP_Lobby) LevelRow))))

(event Custom|SVR_SetViewTarget_Char
  (Game|Player|SetViewTargetwithBlend (Variables|/Script/Engine.ChildActorComponent|GetChildActor (Variables|/Game/Gameplay/Lobby/BP_LobbyPlayer.BP_LobbyPlayer_C|GetViewTarget (Variables|Default|GetLobbyCharacter))) 0.5 "VTBlend_Linear" 0.0 false))

(event Custom|SVR_UpdateSelectedChar
  (params (Profile :type S%20Player%20Profile%20Structure))
  (bind _output_get (Variables|Default|SetPlayerProfile Profile))
  (bind _asbp_mgm (Utilities|Casting|CastToBP_MGM (Game|GetGameMode)))
  (Default|UpdateCharforController _asbp_mgm self _output_get))

(event EventBeginPlay
  (if (Pawn|IsLocalController)
    (Variables|Default|SetbShowMouseCursor true)
    (Input|SetInputModeUIOnly self 0 "DoNotLock" false)))

(fn ConstructionScript)

(fn UIShowLobbyMenu
  (Utilities|IsValid (Variables|Default|GetWBP_Lobby)
    (:Is%20Valid
      _)
    (:Is%20Not%20Valid
      (bind _returnvalue (UserInterface|CreateWidget "/Game/Widgets/WBP_LobbyMenu.WBP_LobbyMenu_C" self))
      (Variables|Default|SetWBP_Lobby _returnvalue)))
  (UserInterface|Viewport|AddtoViewport (Variables|Default|GetWBP_Lobby) 0)
  (Networking|SwitchHasAuthority
    (:Authority
      (Game|Player|SetViewTargetwithBlend (Pawn|GetControlledPawn) 0.5 "VTBlend_Linear" 0.0 false))
    (:Remote
      (CallFunction|SVRSetViewTarget)))
  (return))

(fn LoadSaveGame
  (bind _returnvalue (SaveGame|DoesSaveGameExist (LocalVariables|GetLcl_SlotName)))
  (if _returnvalue
    _
    (else
      (bind _returnvalue_2 (SaveGame|CreateSaveGameObject "/Game/SaveData/SG_PlayerProfile.SG_PlayerProfile_C"))
      (SaveGame|SaveGametoSlot _returnvalue_2 (LocalVariables|GetLcl_SlotName))))
  (bind _returnvalue_3 (SaveGame|LoadGamefromSlot (LocalVariables|GetLcl_SlotName)))
  (bind _assg_player_profile (Utilities|Casting|CastToSG_PlayerProfile _returnvalue_3))
  (Variables|Default|SetPlayerProfile (Variables|/Game/SaveData/SG_PlayerProfile.SG_PlayerProfile_C|GetPlayerProfile _assg_player_profile))
  (return))

(fn UIShowLoading
  (Viewport|RemoveAllWidgets)
  (Utilities|IsValid (Variables|Default|GetWBP_Loading)
    (:Is%20Valid
      _)
    (:Is%20Not%20Valid
      (bind _returnvalue (UserInterface|CreateWidget "/Game/Widgets/WBP_Loading.WBP_Loading_C" self))
      (Variables|Default|SetWBP_Loading _returnvalue)))
  (UserInterface|Viewport|AddtoViewport (Variables|Default|GetWBP_Loading) 0)
  (return))

(fn UIShowCharacterMenu
  (Utilities|IsValid (Variables|Default|GetWBP_Character)
    (:Is%20Valid
      _)
    (:Is%20Not%20Valid
      (bind _returnvalue (UserInterface|CreateWidget "/Game/Widgets/WBP_CharacterMenu.WBP_CharacterMenu_C" self))
      (Variables|Default|SetWBP_Character _returnvalue)))
  (UserInterface|Viewport|AddtoViewport (Variables|Default|GetWBP_Character) 0)
  (Networking|SwitchHasAuthority
    (:Authority
      (Game|Player|SetViewTargetwithBlend (Variables|/Script/Engine.ChildActorComponent|GetChildActor (Variables|/Game/Gameplay/Lobby/BP_LobbyPlayer.BP_LobbyPlayer_C|GetViewTarget (Variables|Default|GetLobbyCharacter))) 0.5 "VTBlend_Linear" 0.0 false))
    (:Remote
      (CallFunction|SVRSetViewTargetChar)))
  (return))

(fn SaveSelectedCharacter
  (params (RowName :type Name) (Class :type Actor%20Class%20Reference))
  (Variables|Default|SetPlayerProfile (Utilities|Struct|MakeS_PlayerProfile RowName Class))
  (Utilities|IsValid (Variables|Default|GetSG_PlayerProfile)
    (:Is%20Valid
      _)
    (:Is%20Not%20Valid
      (bind _returnvalue (SaveGame|CreateSaveGameObject "/Game/SaveData/SG_PlayerProfile.SG_PlayerProfile_C"))
      (Variables|Default|SetSG_PlayerProfile _returnvalue)))
  (Variables|/Game/SaveData/SG_PlayerProfile.SG_PlayerProfile_C|SetPlayerProfile (Variables|Default|GetSG_PlayerProfile) (Variables|Default|GetPlayerProfile))
  (SaveGame|SaveGametoSlot (Variables|Default|GetSG_PlayerProfile) "PlayerProfile")
  (CallFunction|SVRUpdateSelectedChar (Variables|Default|GetPlayerProfile))
  (return))