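; BP_GPPC is a player controller that sets up the local player's HUD, input and session exit.
; On BeginPlay, if local, it clears widgets, shows WBP_HUD, switches to game-only input and adds the default Enhanced Input mapping context.
; Its events re-enable pawn input, trigger the HUD countdown or make the HUD visible.
; EndClientSession clears the GameInstance's multiplayer pause flag, destroys the session and opens the main menu map.
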(event Custom|Countdown
  (Default|Countdown (Variables|Default|GetWBP_HUD)))

(event Custom|ShowHUD
  (Widget|SetVisibility (Variables|Default|GetWBP_HUD) "Visible"))

(event Custom|EnableAllInput
  (Input|EnableInput (Pawn|GetControlledPawn) self))

(event Custom|EndClientSession
  (bind _asbp_game_instance (Utilities|Casting|CastToBP_GameInstance (Game|GetGameInstance)))
  (Variables|/Game/Framework/BP_GameInstance.BP_GameInstance_C|SetMP_Paused _asbp_game_instance false)
  (|DestroySession self
    (:then
      (Game|OpenLevel(byName) "MainMenuMap "))))

(event EventBeginPlay
  (bind _returnvalue (PlayerController|LocalPlayerSubsystems|GetEnhancedInputLocalPlayerSubsystem))
  (if (Pawn|IsLocalController)
    (Viewport|RemoveAllWidgets)
    (CallFunction|UIShowHUD)
    (Input|SetInputModeGameOnly self false)
    (Variables|Default|SetbShowMouseCursor false)
    (Utilities|IsValid _returnvalue
      (:Is%20Valid
        (Input|AddMappingContext _returnvalue "/Game/Input/IMC_Default.IMC_Default" 0 "(bIgnoreAllPressedKeysUntilRelease=True,bForceImmediately=False,bNotifyUserSettings=False)")))))

(fn ConstructionScript)

(fn UIShowHUD
  (Utilities|IsValid (Variables|Default|GetWBP_HUD)
    (:Is%20Valid
      _)
    (:Is%20Not%20Valid
      (bind _returnvalue (UserInterface|CreateWidget "/Game/Widgets/WBP_HUD.WBP_HUD_C" self))
      (Variables|Default|SetWBP_HUD _returnvalue)))
  (UserInterface|Viewport|AddtoViewport (Variables|Default|GetWBP_HUD) 0)
  (return))